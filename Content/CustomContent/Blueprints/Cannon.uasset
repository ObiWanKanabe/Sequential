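; Player-controlled cannon that drives along the camera's forward vector with spinning wheels, aims by controller yaw and pitch, and fires Cannonballs.
; Launch spawns a Cannonball at the Arrow using control rotation, then clears CanShoot for a short delay, blocking movement, aiming and firing.
; A separately gated Recoil1 timeline offsets both spring arms along the Arrow's flattened forward vector.
; Both offsets share StartPosHead, which BeginPlay sets from SpringArm then overwrites with SpringArmBase.
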(event `self.ReceiveBeginPlay`
  ;[1 1 1] StartingPositionsRelative
  (set `self.StartPosHead` (`SceneComponent.GetRelativeTransform` (`self.SpringArm`)))
  (set `self.StartPosHead` (`SceneComponent.GetRelativeTransform` (`self.SpringArmBase`))))

(event `InputAxis|Forward`
  (params (AxisValue :type "Float (single-precision)"))
  ;[1 1 1] Input
  (if (`self.CanShoot`)
    (`SceneComponent.K2_AddWorldTransform` (`self.DefaultSceneRoot`) (`KismetMathLibrary.Conv_VectorToTransform` (* (`SceneComponent.GetForwardVector` (`self.Camera`)) AxisValue)) false false)
    (bind _result (`/Engine/EditorBlueprintResources/StandardMacros.NegateFloat` AxisValue)
      (:`  `
        (bind _returnvalue (`KismetMathLibrary.MakeRotator` 0.0 0.0 _result))
        (`SceneComponent.K2_AddLocalRotation` (`self.CannonWheel1`) _returnvalue false false)
        (`SceneComponent.K2_AddLocalRotation` (`self.CannonWheel2`) _returnvalue false false)))))

(event `InputAxis|Left/Right`
  (params (AxisValue :type "Float (single-precision)"))
  ;[1 1 1] Input
  (if (`self.CanShoot`)
    (`self.AddControllerYawInput` AxisValue)))

(event `InputAxis|Up/Down`
  (params (AxisValue :type "Float (single-precision)"))
  ;[1 1 1] Input
  (if (`self.CanShoot`)
    (`self.AddControllerPitchInput` AxisValue)))

(event `InputAction|Launch`
  (params (Key :type "Key Structure"))
  ;[1 1 1] Fire Projectile
  (:`Pressed`
    (if (`self.CanShoot`)
      (`|SpawnActorFromClass` "/Game/CustomContent/Blueprints/Cannonball.Cannonball_C" (`KismetMathLibrary.MakeTransform` (`SceneComponent.K2_GetComponentLocation` (`self.Arrow`)) (`self.GetControlRotation`)) "Undefined" "OverrideRootScale" null null)
      (set `self.CanShoot` false)
      (`KismetSystemLibrary.Delay` 1.0)
      (set `self.CanShoot` true))))

(event `InputAction|Launch`
  (params (Key :type "Key Structure"))
  ;[1 1 1] CannonRecoil
  (:`Pressed`
    (if (not (`self.IsShooting`))
      (bind (_direction _recoilfloat) (`Timeline|Recoil1` :!via `PlayFromStart`)
        (:`Update`
          (set `self.IsShooting` true)
          (bind _returnvalue (+ (* (`KismetMathLibrary.MakeVector` (.x (`SceneComponent.GetForwardVector` (`self.Arrow`))) (.y (`SceneComponent.GetForwardVector` (`self.Arrow`)))) _recoilfloat) (.location (`self.StartPosHead`))))
          (`SceneComponent.K2_SetRelativeLocation` (`self.SpringArm`) _returnvalue true false)
          (`SceneComponent.K2_SetRelativeLocation` (`self.SpringArmBase`) _returnvalue false false))
        (:`Finished`
          (set `self.IsShooting` false))))))

(fn `UserConstructionScript`)