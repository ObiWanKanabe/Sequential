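; Player controller that switches the player's possession between MyCharacter and the CannonHead and CannonBase actors.
; The CannonHead and CannonBase inputs each toggle control of their part or return to the character, and Esc always returns to the character.
; Two booleans track the possessed part, and each target is the first actor found of its class via GetAllActorsOfClass.
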(event `InputAction|CannonHead` :consume false :overrideparent false
  (params (Key :type "Key Structure"))
  (:`Pressed`
    (if (`self.HeadPosses`)
      (bind _outactors (`GameplayStatics.GetAllActorsOfClass` "/Game/Custom_Content/Character/Blueprints/MyCharacter.MyCharacter_C"))
      (`self.Possess` (`|GetArrayItem` _outactors))
      (set `self.HeadPosses` false)
      (set `self.BasePosses` false)
      (else
        (set `self.HeadPosses` true)
        (set `self.BasePosses` false)
        (bind _outactors_2 (`GameplayStatics.GetAllActorsOfClass` "/Game/Custom_Content/BluePrints/CannonRoom/CannonHead.CannonHead_C"))
        (`self.Possess` (`|GetArrayItem` _outactors_2))))))

(event `InputAction|CannonBase` :consume false :overrideparent false
  (params (Key :type "Key Structure"))
  (:`Pressed`
    (if (`self.BasePosses`)
      (bind _outactors (`GameplayStatics.GetAllActorsOfClass` "/Game/Custom_Content/Character/Blueprints/MyCharacter.MyCharacter_C"))
      (`self.Possess` (`|GetArrayItem` _outactors))
      (set `self.HeadPosses` false)
      (set `self.BasePosses` false)
      (else
        (set `self.BasePosses` true)
        (set `self.HeadPosses` false)
        (bind _outactors_2 (`GameplayStatics.GetAllActorsOfClass` "/Game/Custom_Content/BluePrints/CannonRoom/CannonBase.CannonBase_C"))
        (`self.Possess` (`|GetArrayItem` _outactors_2))))))

(event `InputAction|Esc`
  (params (Key :type "Key Structure"))
  (:`Pressed`
    (set `self.HeadPosses` false)
    (set `self.BasePosses` false)
    (bind _outactors (`GameplayStatics.GetAllActorsOfClass` "/Game/Custom_Content/Character/Blueprints/MyCharacter.MyCharacter_C"))
    (`self.Possess` (`|GetArrayItem` _outactors))))

(fn `UserConstructionScript`)