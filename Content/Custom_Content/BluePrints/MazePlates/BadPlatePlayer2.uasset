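; BadPlatePlayer2 is a maze trap plate, named for player 2, that sends any actor stepping on it back to a respawn location.
; When an actor enters its Box, the plate turns red, moves that actor to RespawnLocation without filtering by player, and plays a failure sound.
; Leaving the Box restores white after a short delay, using a dynamic material instance created on the Plate in the construction script.
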(event `self.Box.OnComponentBeginOverlap`
  (params (OverlappedComponent :type "PrimitiveComponent Object Reference") (OtherActor :type "Actor Object Reference") (OtherComp :type "PrimitiveComponent Object Reference") (OtherBodyIndex :type Integer) (bFromSweep :type Boolean) (SweepResult :type "HitResult Structure (by ref)"))
  ;[1 1 1] Changing Colour
  (`MaterialInstanceDynamic.SetVectorParameterValue` (`self.Dynamic Material`) "Color" (struct :`R` 0.78125 :`B` 0.007105 :`A` 1.0))
  (`self.K2_SetActorTransform` OtherActor (`KismetMathLibrary.Conv_VectorToTransform` (`self.Respawn location`)) false false)
  (`GameplayStatics.PlaySound2D` "/Game/Custom_Content/Audio/Failure.Failure" 1.0 1.0 0.0 null null))

(event `self.Box.OnComponentEndOverlap`
  (params (OverlappedComponent :type "PrimitiveComponent Object Reference") (OtherActor :type "Actor Object Reference") (OtherComp :type "PrimitiveComponent Object Reference") (OtherBodyIndex :type Integer))
  ;[1 1 1] Changing Colour
  (`KismetSystemLibrary.Delay` 0.5)
  (`MaterialInstanceDynamic.SetVectorParameterValue` (`self.Dynamic Material`) "Color" (struct :`R` 1.0 :`G` 1.0 :`B` 1.0 :`A` 1.0)))

(fn `UserConstructionScript`
  (bind _returnvalue (`PrimitiveComponent.CreateDynamicMaterialInstance` (`self.Plate`) 0 null "None"))
  (set `self.Dynamic Material` _returnvalue))