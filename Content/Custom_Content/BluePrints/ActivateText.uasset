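; ActivateText is a proximity text actor that shows its TextRender only while something overlaps its Box.
; The text starts hidden on BeginPlay, and the Box's begin and end overlap events toggle its visibility without filtering the overlapping actor.
; Every Tick rotates the text so its forward X axis points at the world origin, as the target location is a fixed zero vector.
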(event `self.ReceiveBeginPlay`
  (`SceneComponent.SetVisibility` (`self.TextRender`) false false))

(event `self.ReceiveTick`
  (params (DeltaSeconds :type "Float (single-precision)"))
  (`SceneComponent.K2_SetWorldRotation` (`self.TextRender`) (`KismetMathLibrary.MakeRotFromX` (`KismetMathLibrary.NegateVector` (- (`SceneComponent.K2_GetComponentLocation` (`self.TextRender`)) (0.0 0.0 0.0)))) false false))

(event `self.Box.OnComponentBeginOverlap`
  (params (OverlappedComponent :type "PrimitiveComponent Object Reference") (OtherActor :type "Actor Object Reference") (OtherComp :type "PrimitiveComponent Object Reference") (OtherBodyIndex :type Integer) (bFromSweep :type Boolean) (SweepResult :type "HitResult Structure (by ref)"))
  (`SceneComponent.SetVisibility` (`self.TextRender`) true false))

(event `self.Box.OnComponentEndOverlap`
  (params (OverlappedComponent :type "PrimitiveComponent Object Reference") (OtherActor :type "Actor Object Reference") (OtherComp :type "PrimitiveComponent Object Reference") (OtherBodyIndex :type Integer))
  (`SceneComponent.SetVisibility` (`self.TextRender`) false false))

(fn `UserConstructionScript`)