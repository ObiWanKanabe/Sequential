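; Cannonball projectile actor for the cannon room, driven by ProjectileMovement and RotatingMovement components and removing itself after it stops or hits hard.
; When the projectile stops, it zeroes its rotation rate and destroys itself after a brief delay.
; Collision hits with a large enough normal impulse play a clang sound at the world origin, not the impact point, then destroy the actor after a short delay.
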(event `self.ProjectileMovement.OnProjectileStop`
  (params (ImpactResult :type "HitResult Structure (by ref)"))
  (set `RotatingMovementComponent.RotationRate` (struct) (`self.RotatingMovement`))
  (`KismetSystemLibrary.Delay` 0.1)
  (`self.K2_DestroyActor`))

(event `self.Collision.OnComponentHit`
  (params (HitComponent :type "PrimitiveComponent Object Reference") (OtherActor :type "Actor Object Reference") (OtherComp :type "PrimitiveComponent Object Reference") (NormalImpulse :type "Vector Structure") (Hit :type "HitResult Structure (by ref)"))
  (if (> (`KismetMathLibrary.VSize` NormalImpulse) 10000.0)
    (`GameplayStatics.PlaySoundAtLocation` "/Game/Custom_Content/Audio/LightClang.LightClang" (0.0 0.0 0.0) (struct) 1.0 1.0 0.0 null null null)
    (`KismetSystemLibrary.Delay` 0.5)
    (`self.K2_DestroyActor`)))

(fn `UserConstructionScript`)