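; Player-controlled cannon base that turns, slides sideways along world Y and plays a recoil when fired.
; Turn and MoveRight drive controller yaw and spring arm offset, both locked during the one-second CanShoot cooldown started by Jump or Launch.
; The same inputs play a recoil timeline that shifts the spring arm along the arrow's flattened forward vector from a resting position cached on Tick.
; No projectile is spawned here.
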(event `self.ReceiveTick`
  (params (DeltaSeconds :type "Float (single-precision)"))
  ;[1 1 1] Starting Positions Relative
  (if (not (`self.IsShooting`))
    (set `self.StartPosBase` (.location (`SceneComponent.GetRelativeTransform` (`self.SpringArm`))))))

(event `InputAxis|Turn`
  (params (AxisValue :type "Float (single-precision)"))
  ;[1 1 1] Input
  (if (`self.CanShoot`)
    (`self.AddControllerYawInput` AxisValue)))

(event `InputAxis|MoveRight`
  (params (AxisValue :type "Float (single-precision)"))
  ;[1 1 1] Input
  (if (`self.CanShoot`)
    (bind _result (`/Engine/EditorBlueprintResources/StandardMacros.NegateFloat` AxisValue)
      (:`  `
        (`SceneComponent.K2_AddWorldOffset` (`self.SpringArm`) (`KismetMathLibrary.MakeVector` 0.0 (* 3.0 _result)) false false)))))

(event `InputAction|Jump`
  (params (Key :type "Key Structure"))
  ;[1 1 1] Fire Projectile
  (:`Pressed`
    (if (`self.CanShoot`) :!label _label
      (set `self.CanShoot` false)
      (`KismetSystemLibrary.Delay` 1.0)
      (set `self.CanShoot` true))))

(event `InputAction|Launch`
  (params (Key :type "Key Structure"))
  ;[1 1 1] Fire Projectile
  (:`Pressed`
    (goto _label)))

(event `InputAction|Jump`
  (params (Key :type "Key Structure"))
  ;[1 1 1] CannonRecoil
  (:`Pressed`
    (if (not (`self.IsShooting`)) :!label _label_2
      (bind (_direction _recoilfloat) (`Timeline|Timeline_0` :!via `PlayFromStart`)
        (:`Update`
          (set `self.IsShooting` true)
          (`SceneComponent.K2_SetRelativeLocation` (`self.SpringArm`) (+ (* (`KismetMathLibrary.MakeVector` (.x (`SceneComponent.GetForwardVector` (`self.Arrow`))) (.y (`SceneComponent.GetForwardVector` (`self.Arrow`)))) _recoilfloat) (`self.StartPosBase`)) true false))
        (:`Finished`
          (set `self.IsShooting` false))))))

(event `InputAction|Launch`
  (params (Key :type "Key Structure"))
  ;[1 1 1] CannonRecoil
  (:`Pressed`
    (goto _label_2)))

(fn `UserConstructionScript`)