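; Cannon room target basket that moves while active and completes when a Cannonball enters its InsideCollision.
; Tick offsets it per axis at Speed using direction flags, with both directions tested against the same start-plus-Bounds point, so it heads there rather than patrolling a range.
; Any overlap plays the success sound; a Cannonball is then destroyed, the basket marked complete and inactive, and its mesh and collision components removed.
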(event `Destroy`
  ;[1 1 1] Comment
  (`ActorComponent.K2_DestroyComponent` (`self.StaticMesh`))
  (`ActorComponent.K2_DestroyComponent` (`self.InsideCollision`)))

(event `self.InsideCollision.OnComponentBeginOverlap`
  (params (OverlappedComponent :type "PrimitiveComponent Object Reference") (OtherActor :type "Actor Object Reference") (OtherComp :type "PrimitiveComponent Object Reference") (OtherBodyIndex :type Integer) (bFromSweep :type Boolean) (SweepResult :type "HitResult Structure (by ref)"))
  ;[1 1 1] Comment
  (`GameplayStatics.PlaySound2D` "/Game/Custom_Content/Audio/Success.Success" 1.0 1.0 0.0 null null)
  (bind _ascannonball (cast `/Game/Custom_Content/BluePrints/CannonRoom/Cannonball` OtherActor))
  (`self.K2_DestroyActor` _ascannonball)
  (set `self.IsComplete` true)
  (set `self.IsActive` false)
  (`self.Destroy`))

(event `self.ReceiveBeginPlay`
  ;[1 1 1] Set Initial Position
  (set `self.InitPos` (`self.K2_GetActorLocation`)))

(event `self.ReceiveTick`
  (params (DeltaSeconds :type "Float (single-precision)"))
  (bind _returnvalue (`KismetMathLibrary.MakeVector` 0.0 0.0 (* (.z (`self.Speed`)) DeltaSeconds)))
  (bind _returnvalue_2 (`KismetMathLibrary.MakeVector` 0.0 (* (.y (`self.Speed`)) DeltaSeconds)))
  (bind _returnvalue_3 (`KismetMathLibrary.MakeVector` (* (.x (`self.Speed`)) DeltaSeconds)))
  ;[1 1 1] Positive Y Movement
  (if (`self.IsActive`)
    (`|ExecutionSequence`
      (:`then_0`
        (if (and (`self.IsMovingY`) (< (.y (`self.K2_GetActorLocation`)) (.y (+ (`self.Bounds+`) (`self.InitPos`)))))
          (`self.K2_AddActorWorldOffset` _returnvalue_2)
          (else
            (set `self.IsMovingY` false))))
      (:`then_1`
        ;[1 1 1] Negative Y Movement
        (if (and (== (`self.IsMovingY`) false) (> (.y (`self.K2_GetActorLocation`)) (.y (+ (`self.InitPos`) (`self.Bounds-`)))))
          (`self.K2_AddActorWorldOffset` (`KismetMathLibrary.NegateVector` _returnvalue_2))
          (else
            (set `self.IsMovingY` true))))
      (:`then_2`
        ;[1 1 1] Positive X Movement
        (if (and (`self.IsMovingX`) (< (.x (`self.K2_GetActorLocation`)) (.x (+ (`self.Bounds+`) (`self.InitPos`)))))
          (`self.K2_AddActorWorldOffset` _returnvalue_3)
          (else
            (set `self.IsMovingX` false))))
      (:`then_3`
        ;[1 1 1] Negative X Movement
        (if (and (== (`self.IsMovingX`) false) (> (.x (`self.K2_GetActorLocation`)) (.x (+ (`self.InitPos`) (`self.Bounds-`)))))
          (`self.K2_AddActorWorldOffset` (`KismetMathLibrary.NegateVector` _returnvalue_3))
          (else
            (set `self.IsMovingX` true))))
      (:`then_4`
        ;[1 1 1] Positive Z Movement
        (if (and (`self.IsMovingZ`) (< (.z (`self.K2_GetActorLocation`)) (.z (+ (`self.Bounds+`) (`self.InitPos`)))))
          (`self.K2_AddActorWorldOffset` _returnvalue)
          (else
            (set `self.IsMovingZ` false))))
      (:`then_5`
        ;[1 1 1] Negative Z Movement
        (if (and (== (`self.IsMovingZ`) false) (> (.z (`self.K2_GetActorLocation`)) (.z (+ (`self.InitPos`) (`self.Bounds-`)))))
          (`self.K2_AddActorWorldOffset` (`KismetMathLibrary.NegateVector` _returnvalue))
          (else
            (set `self.IsMovingZ` true)))))))

(fn `UserConstructionScript`)