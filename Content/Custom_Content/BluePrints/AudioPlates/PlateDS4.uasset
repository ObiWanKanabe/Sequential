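; PlateDS4 is an audio plate actor that plays a musical note while something overlaps its collision, likely D#4 given its name.
; Begin overlap starts the Note audio from the beginning and sets WasPressed, which is never cleared here; end overlap stops the note.
; Each action goes through a Request event that forwards to the event doing the work: PlaySound, StopSound or Activate.
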(event `RequestActivate`
  (`self.Activate`))

(event `Activate`
  (set `self.wasPressed` true))

(event `PlaySound`
  (`AudioComponent.Play` (`self.Note`) 0.0))

(event `self.Collision.OnComponentBeginOverlap`
  (params (OverlappedComponent :type "PrimitiveComponent Object Reference") (OtherActor :type "Actor Object Reference") (OtherComp :type "PrimitiveComponent Object Reference") (OtherBodyIndex :type Integer) (bFromSweep :type Boolean) (SweepResult :type "HitResult Structure (by ref)"))
  (`self.RequestPlaySound`)
  (`self.RequestActivate`))

(event `RequestPlaySound`
  (`self.PlaySound`))

(event `StopSound`
  (`AudioComponent.Stop` (`self.Note`)))

(event `self.Collision.OnComponentEndOverlap`
  (params (OverlappedComponent :type "PrimitiveComponent Object Reference") (OtherActor :type "Actor Object Reference") (OtherComp :type "PrimitiveComponent Object Reference") (OtherBodyIndex :type Integer))
  (`self.RequestStopSound`))

(event `RequestStopSound`
  (`self.StopSound`))

(fn `UserConstructionScript`)