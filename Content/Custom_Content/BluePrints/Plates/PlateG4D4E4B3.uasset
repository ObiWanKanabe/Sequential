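; Musical plate actor that plays a sequence of four notes, likely G4, D4, E4 and B3 judging by its name, when something overlaps its Collision component.
; The overlap calls RequestPlaySound, which forwards to PlaySound.
; PlaySound starts four audio components one second apart through nested IsPlaying checks, so the chain stops at any note that is already playing.
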(event `PlaySound`
  (bind _note4 (`self.Note4`))
  (bind _note2 (`self.Note2`))
  (bind _note3 (`self.Note3`))
  (bind _note (`self.Note`))
  (if (not (`AudioComponent.IsPlaying` _note))
    (`AudioComponent.Play` _note 0.0)
    (`KismetSystemLibrary.Delay` 1.0)
    (if (not (`AudioComponent.IsPlaying` _note2))
      (`AudioComponent.Play` _note2 0.0)
      (`KismetSystemLibrary.Delay` 1.0)
      (if (not (`AudioComponent.IsPlaying` _note3))
        (`AudioComponent.Play` _note3 0.0)
        (`KismetSystemLibrary.Delay` 1.0)
        (if (not (`AudioComponent.IsPlaying` _note4))
          (`AudioComponent.Play` _note4 0.0))))))

(event `self.Collision.OnComponentBeginOverlap`
  (params (OverlappedComponent :type "PrimitiveComponent Object Reference") (OtherActor :type "Actor Object Reference") (OtherComp :type "PrimitiveComponent Object Reference") (OtherBodyIndex :type Integer) (bFromSweep :type Boolean) (SweepResult :type "HitResult Structure (by ref)"))
  (`self.RequestPlaySound`))

(event `self.Collision.OnComponentEndOverlap`
  (params (OverlappedComponent :type "PrimitiveComponent Object Reference") (OtherActor :type "Actor Object Reference") (OtherComp :type "PrimitiveComponent Object Reference") (OtherBodyIndex :type Integer)))

(event `RequestPlaySound`
  (`self.PlaySound`))

(fn `UserConstructionScript`)